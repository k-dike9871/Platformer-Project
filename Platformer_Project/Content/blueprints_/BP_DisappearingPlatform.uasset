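; A platform that turns red when stepped on, vanishes, then comes back.
; A box trigger overlap by a BP_Base actor swaps the mesh material to red, then after a short delay hides the mesh and disables its collision.
; Any actor leaving the box starts a longer delay that restores the wall material, visibility and collision, with no class check.
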(event `self.Box.OnComponentBeginOverlap`
  (params (OverlappedComponent :type "PrimitiveComponent Object Reference") (OtherActor :type "Actor Object Reference") (OtherComp :type "PrimitiveComponent Object Reference") (OtherBodyIndex :type Integer) (bFromSweep :type Boolean) (SweepResult :type "HitResult Structure (by ref)"))
  (cast `/Game/blueprints_/BP_Base` OtherActor)
  (`PrimitiveComponent.SetMaterial` (`self.StaticMesh`) 0 "/Game/LPSDeluxe2TropicalEnvironment/LPSD2_Materials/Materials/Master_Color_Instances/MI_Color_Red.MI_Color_Red")
  (`KismetSystemLibrary.Delay` 2.0)
  (`SceneComponent.SetVisibility` (`self.StaticMesh`) false false)
  (`PrimitiveComponent.SetCollisionEnabled` (`self.StaticMesh`) "NoCollision"))

(event `self.Box.OnComponentEndOverlap`
  (params (OverlappedComponent :type "PrimitiveComponent Object Reference") (OtherActor :type "Actor Object Reference") (OtherComp :type "PrimitiveComponent Object Reference") (OtherBodyIndex :type Integer))
  (`KismetSystemLibrary.Delay` 3.0)
  (`PrimitiveComponent.SetMaterial` (`self.StaticMesh`) 0 "/Game/StarterContent/Materials/M_Basic_Wall.M_Basic_Wall")
  (`SceneComponent.SetVisibility` (`self.StaticMesh`) true false)
  (`PrimitiveComponent.SetCollisionEnabled` (`self.StaticMesh`) "QueryAndPhysics"))

(fn `UserConstructionScript`)