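; BP_Damage is a trap actor that damages BP_Base characters on contact with its Box component.
; On overlap, it casts the other actor's instigator to BP_Base, blinks it and launches it upward and against the trap's forward vector.
; It then decreases and checks health, repeating after DurationBeforeDamage while the TouchingTrap flag stays set.
; End overlap clears the flag to stop the delay loop.
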(event `self.Box.OnComponentBeginOverlap`
  (params (OverlappedComponent :type "PrimitiveComponent Object Reference") (OtherActor :type "Actor Object Reference") (OtherComp :type "PrimitiveComponent Object Reference") (OtherBodyIndex :type Integer) (bFromSweep :type Boolean) (SweepResult :type "HitResult Structure (by ref)"))
  (bind _asbp_base (cast `/Game/blueprints_/BP_Base` (`self.GetInstigator` OtherActor)))
  (`/Game/blueprints_/BP_Base.Blink` _asbp_base)
  (`Character.LaunchCharacter` _asbp_base (`KismetMathLibrary.MakeVector` (* (.x (`self.GetActorForwardVector`)) -750.0) (* (.y (`self.GetActorForwardVector`)) -750.0) 750.0) false false)
  (set `self.Touching Trap` true)
  (`/Game/blueprints_/BP_Base.Decrease Health` _asbp_base 1.0 :!label _label)
  (`/Game/blueprints_/BP_Base.Check Health` _asbp_base)
  (`KismetSystemLibrary.Delay` (`self.Duration Before Damage`))
  (if (`self.Touching Trap`)
    (goto _label)))

(event `self.Box.OnComponentEndOverlap`
  (params (OverlappedComponent :type "PrimitiveComponent Object Reference") (OtherActor :type "Actor Object Reference") (OtherComp :type "PrimitiveComponent Object Reference") (OtherBodyIndex :type Integer))
  (cast `/Game/blueprints_/BP_Base` (`self.GetInstigator` OtherActor))
  (set `self.Touching Trap` false))

(fn `UserConstructionScript`)