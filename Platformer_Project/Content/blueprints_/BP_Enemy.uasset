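; BP_Enemy is a patrolling enemy character that hurts the player on contact and can be killed by a head hit.
; It loops AI MoveTo through two to four move points with random pauses, continuing even when a move fails.
; The player's EnemyHit component overlapping Head triggers a one-time death that stops movement, ignores Pawn and Camera collision, bounces the player and awards coins.
; Sphere overlap damages the player while the enemy lives.
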(event `self.ReceiveBeginPlay`
  (`self.Walking`))

(event `Walking`
  (`|AIMoveTo` self (0.0 0.0 0.0) (`self.MovePoint1`)
    (:`OnSuccess`
      _)
    (:`OnFail`
      _))
  (`KismetSystemLibrary.Delay` (`KismetMathLibrary.RandomFloatInRange` 1.0 3.0))
  (if (not (`self.Dead?`))
    (`|AIMoveTo` self (0.0 0.0 0.0) (`self.MovePoint2`)
      (:`OnSuccess`
        _)
      (:`OnFail`
        _))
    (`KismetSystemLibrary.Delay` (`KismetMathLibrary.RandomFloatInRange` 1.0 3.0))
    (`/Engine/EditorBlueprintResources/StandardMacros.IsValid` (`self.MovePoint3`)
      (:`Is Valid`
        (`|AIMoveTo` self (0.0 0.0 0.0) (`self.MovePoint3`)
          (:`OnSuccess`
            _)
          (:`OnFail`
            _))
        (`KismetSystemLibrary.Delay` (`KismetMathLibrary.RandomFloatInRange` 1.0 3.0))
        (`/Engine/EditorBlueprintResources/StandardMacros.IsValid` (`self.MovePoint4`)
          (:`Is Valid`
            (`|AIMoveTo` self (0.0 0.0 0.0) (`self.MovePoint4`)
              (:`OnSuccess`
                _)
              (:`OnFail`
                _))
            (`KismetSystemLibrary.Delay` (`KismetMathLibrary.RandomFloatInRange` 1.0 3.0)))
          (:`Is Not Valid`
            _)))
      (:`Is Not Valid`
        _))
    (if (not (`self.Dead?`))
      (`self.Walking`))))

(event `self.Head.OnComponentBeginOverlap`
  (params (OverlappedComponent :type "PrimitiveComponent Object Reference") (OtherActor :type "Actor Object Reference") (OtherComp :type "PrimitiveComponent Object Reference") (OtherBodyIndex :type Integer) (bFromSweep :type Boolean) (SweepResult :type "HitResult Structure (by ref)"))
  (bind _asbp_base (cast `/Game/blueprints_/BP_Base` OtherActor))
  (set `self.Player REF` _asbp_base)
  (if (== OtherComp (`/Game/blueprints_/BP_Base.EnemyHit` _asbp_base))
    (`self.Kill`)))

(event `Kill`
  (bind _player_ref (`self.Player REF`))
  (`/Engine/EditorBlueprintResources/StandardMacros.DoOnce` false
    (:`Completed`
      (`SkeletalMeshComponent.PlayAnimation` (`self.Mesh`) "/Game/Characters/Enemy/Animations/Falling_Back_Death.Falling_Back_Death" false)
      (`PrimitiveComponent.SetCollisionResponseToChannel` (`self.CapsuleComponent`) "ECC_Pawn" "ECR_Ignore")
      (`PrimitiveComponent.SetCollisionResponseToChannel` (`self.Mesh`) "ECC_Pawn" "ECR_Ignore")
      (`PrimitiveComponent.SetCollisionResponseToChannel` (`self.CapsuleComponent`) "ECC_Camera" "ECR_Ignore")
      (`PrimitiveComponent.SetCollisionResponseToChannel` (`self.Mesh`) "ECC_Camera" "ECR_Ignore")
      (set `self.Dead?` true)
      (set `CharacterMovementComponent.MaxWalkSpeed` 0.0 (`self.CharacterMovement`))
      (`self.LaunchCharacter` _player_ref (0.0 0.0 500.0) false true)
      (set `/Game/blueprints_/BP_Base.Coins` (+ (`/Game/blueprints_/BP_Base.Coins` _player_ref) 5) _player_ref))))

(event `self.Sphere.OnComponentBeginOverlap`
  (params (OverlappedComponent :type "PrimitiveComponent Object Reference") (OtherActor :type "Actor Object Reference") (OtherComp :type "PrimitiveComponent Object Reference") (OtherBodyIndex :type Integer) (bFromSweep :type Boolean) (SweepResult :type "HitResult Structure (by ref)"))
  (bind _asbp_base (cast `/Game/blueprints_/BP_Base` OtherActor))
  (if (not (`self.Dead?`))
    (`GameplayStatics.ApplyDamage` _asbp_base 1.0)))

(fn `UserConstructionScript`)