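; Coins_BP is a collectible coin pickup that spins in place until collected.
; Tick yaws CoinMesh by RotationSpeed each frame, without scaling by delta time.
; When the Sphere overlaps an actor whose instigator casts to BP_Base, it increments that object's Coins count, prints the new total and destroys itself.
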(event `self.ReceiveTick`
  (params (DeltaSeconds :type "Float (single-precision)"))
  (`SceneComponent.K2_AddRelativeRotation` (`self.CoinMesh`) (`KismetMathLibrary.MakeRotator` 0.0 0.0 (`self.Rotation Speed`)) false false))

(event `self.Sphere.OnComponentBeginOverlap`
  (params (OverlappedComponent :type "PrimitiveComponent Object Reference") (OtherActor :type "Actor Object Reference") (OtherComp :type "PrimitiveComponent Object Reference") (OtherBodyIndex :type Integer) (bFromSweep :type Boolean) (SweepResult :type "HitResult Structure (by ref)"))
  (bind _asbp_base (cast `/Game/blueprints_/BP_Base` (`self.GetInstigator` OtherActor)))
  (bind _output_get (set `/Game/blueprints_/BP_Base.Coins` (+ (`/Game/blueprints_/BP_Base.Coins` _asbp_base) 1) _asbp_base))
  (`KismetSystemLibrary.PrintString` (`KismetStringLibrary.Conv_IntToString` _output_get))
  (`self.K2_DestroyActor`))

(fn `UserConstructionScript`)