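; BP_Door is a door that opens when enough pressure switches are active at once.
; SwitchActivated and SwitchDeactivated events raise or lower a count of active switches and compare it to the required number.
; Meeting the threshold plays the DoorActivate timeline, which moves the Cube's relative Z position, and falling below it reverses the timeline.
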(event `Switch Activated`
  (`/Engine/EditorBlueprintResources/StandardMacros.IncrementInt` (`self.Pressure Switches Activated`)
    (:`  `
      (if (>= (`self.Pressure Switches Activated`) (`self.Pressure Switches Needed`))
        (bind (_direction _door_position) (`Timeline|Door Activate` :!label _label)
          (:`Update`
            (`SceneComponent.K2_SetRelativeLocation` (`self.Cube`) (`KismetMathLibrary.MakeVector` 0.0 0.0 _door_position) false false)))
        (else
          (goto _label :!via `Reverse`))))))

(event `Switch Deactivated`
  (`/Engine/EditorBlueprintResources/StandardMacros.DecrementInt` (`self.Pressure Switches Activated`)
    (:`  `
      (if (>= (`self.Pressure Switches Activated`) (`self.Pressure Switches Needed`))
        (goto _label)
        (else
          (goto _label :!via `Reverse`))))))

(fn `UserConstructionScript`)