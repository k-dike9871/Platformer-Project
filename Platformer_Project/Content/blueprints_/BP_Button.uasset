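; BP_Button is a pressable button that deactivates the shield on an actor found by class.
; Overlap with a BP_Base actor opens a gate that lets the Interact input through, and leaving closes it.
; The Button Animation macro plays a push sound and lerps the button in and back out on two timelines.
; Both macro outputs fire from timeline updates, so DeactivateShield is called repeatedly during the animation.
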(event `self.ReceiveBeginPlay`
  (bind (_returnvalue_location _returnvalue_rotation _returnvalue_scale) (`KismetMathLibrary.BreakTransform` (`SceneComponent.GetRelativeTransform` (`self.Button`))))
  (set `self.Out Pos` (`KismetMathLibrary.MakeTransform` _returnvalue_location _returnvalue_rotation _returnvalue_scale))
  (set `self.In Pos` (`KismetMathLibrary.MakeTransform` (- _returnvalue_location (0.0 10.0 0.0)) _returnvalue_rotation _returnvalue_scale))
  (`self.EnableInput` (`GameplayStatics.GetPlayerController` 0)))

(event `InputAction|Interact`
  (params (Key :type "Key Structure"))
  ;[1 1 1] Button Interaction
  (:`Pressed`
    (`/Engine/EditorBlueprintResources/StandardMacros.Gate` true :!label _label
      (:`Exit`
        ;[1 1 1] Button Animation
        (`GameplayStatics.PlaySoundAtLocation` "/Game/Audio/240224__xtrgamr__buttonpush_01.240224__xtrgamr__buttonpush_01" (`self.K2_GetActorLocation`) (struct) 1.0 1.0 0.0 null null null)
        (bind (_direction _button_in) (`Timeline|Button In` :!via `PlayFromStart`)
          (:`Update`
            (`SceneComponent.K2_SetRelativeTransform` (`self.Button`) (`KismetMathLibrary.TLerp` (`self.Out Pos`) (`self.In Pos`) _button_in) false false)
            ;[1 1 1] Code To Be Executed
            (bind _returnvalue (`GameplayStatics.GetActorOfClass` "/Game/blueprints_/BP.BP_C"))
            (`/Game/blueprints_/BP.Deactivate Shield` _returnvalue))
          (:`Finished`
            (bind (_direction_2 _button_in_2) (`Timeline|Timeline_0` :!via `ReverseFromEnd`)
              (:`Update`
                (`SceneComponent.K2_SetRelativeTransform` (`self.Button`) (`KismetMathLibrary.TLerp` (`self.Out Pos`) (`self.In Pos`) _button_in_2) false false)
                (bind _returnvalue_2 (`GameplayStatics.GetActorOfClass` "/Game/blueprints_/BP.BP_C"))
                (`/Game/blueprints_/BP.Deactivate Shield` _returnvalue_2)))))))))

(event `self.Box.OnComponentBeginOverlap`
  (params (OverlappedComponent :type "PrimitiveComponent Object Reference") (OtherActor :type "Actor Object Reference") (OtherComp :type "PrimitiveComponent Object Reference") (OtherBodyIndex :type Integer) (bFromSweep :type Boolean) (SweepResult :type "HitResult Structure (by ref)"))
  ;[1 1 1] Button Interaction
  (cast `/Game/blueprints_/BP_Base` OtherActor)
  (goto _label :!via `Open`))

(event `self.Box.OnComponentEndOverlap`
  (params (OverlappedComponent :type "PrimitiveComponent Object Reference") (OtherActor :type "Actor Object Reference") (OtherComp :type "PrimitiveComponent Object Reference") (OtherBodyIndex :type Integer))
  ;[1 1 1] Button Interaction
  (cast `/Game/blueprints_/BP_Base` OtherActor)
  (goto _label :!via `Close`))

(fn `UserConstructionScript`)